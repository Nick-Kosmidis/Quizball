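; Game instance Blueprint for Quizball that holds the player list and tracks whose turn it is.
; AddPlayer appends each player's name and points to PlayerProperties.
; GetPlayerOnTurn returns index 0 for a single player, otherwise 0 or 1 based on the Player1Turn flag.
; ChangeTurn flips that flag, so turn alternation covers only two players.
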(fn AddPlayer
  (params (Properties :type Player%20Properties%20Structure))
  (Utilities|Array|Add (Variables|Default|GetPlayerProperties) (Utilities|Struct|MakePlayerProperties (.name Properties) (.points Properties))))

(fn GetPlayeronTurn
  (if (== (Utilities|Array|Length (Variables|Default|GetPlayerProperties)) 1)
    (return 0)
    (else
      (if (Variables|Default|GetPlayer1Turn)
        (Variables|Default|SetPlayerIndex 0)
        (else
          (Variables|Default|SetPlayerIndex 1)))
      (return (Variables|Default|GetPlayerIndex)))))

(fn ChangeTurn
  (Variables|Default|SetPlayer1Turn (not (Variables|Default|GetPlayer1Turn))))