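; Blueprint utility library for Quizball that gives shortcuts to the game's core objects.
; Getters cast player 0's HUD and pawn, plus the game instance, to their Quizball classes, with an extra validity check on the HUD.
; The current question getter builds on the HUD getter, reading it from the HUD's QuizballQuestion.
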(fn GetQuizballHUD
  (bind _asquizball_hudbp (Utilities|Casting|CastToQuizballHUDBP (HUD|GetHUD (Game|GetPlayerController 0))))
  (Utilities|IsValid _asquizball_hudbp
    (:Is%20Valid
      (return _asquizball_hudbp))))

(fn GetCurrentQuestion
  (return (Variables|/Script/Quizball.QuizballQuestion|GetCurrentQuestion (Variables|/Game/Blueprints/QuizballHUDBP.QuizballHUDBP_C|GetQuizballQuestion (CallFunction|GetQuizballHUD)))))

(fn GetQuizballGameInstance
  (bind _asquizball_game_instance_bp (Utilities|Casting|CastToQuizballGameInstanceBP (Game|GetGameInstance)))
  (return _asquizball_game_instance_bp))

(fn GetQuizballPlayerPawn
  (bind _asplayer_pawn_bp (Utilities|Casting|CastToPlayerPawnBP (Game|Player|GetPlayerPawn 0)))
  (return _asplayer_pawn_bp))